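; Base weapon Blueprint that handles firing and reloading, with ammo tracked as a clip count and a reserve.
; WB_Fire spawns a projectile at the mesh's Muzzle socket, decrements Ammo, and plays a muzzle emitter and attenuated AK47 sound there.
; Reload skips a full clip; otherwise it overwrites Ammo from the reserve, discarding rounds left in the clip, and sets IsReloading on the first player's FPPlayerCharacter.
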(event `WB_Fire`
  (bind _returnvalue (`SceneComponent.GetSocketTransform` (`self.SkeletalMesh`) "Muzzle" "RTS_World"))
  (bind _location (.location _returnvalue))
  (`|SpawnActorFromClass` "/Game/Assets/Weapons/Ammo/Projectile_Base.Projectile_Base_C" _returnvalue "Undefined" "OverrideRootScale" null null)
  (set `self.Ammo` (- (`self.Ammo`) 1))
  (`GameplayStatics.SpawnEmitterAtLocation` "/Game/Assets/Effects/Weapons/BaseMuzzle.BaseMuzzle" _location (.rotation _returnvalue))
  (`GameplayStatics.PlaySoundAtLocation` "/Game/Assets/Sounds/Weapons/AK47.AK47" _location (struct) 1.0 1.0 0.0 "/Game/Assets/Sounds/Weapons/WeaponShotBaseAttenuation.WeaponShotBaseAttenuation" null null))

(fn `Reload`
  (returns (Output_Get :type Boolean) (Output_Get1 :type Boolean))
  (if (not (== (`self.ClipSize`) (`self.Ammo`)))
    (if (> (`self.MaxAmmo`) (`self.ClipSize`))
      (set `self.Ammo` (`self.ClipSize`))
      (set `self.MaxAmmo` (- (`self.MaxAmmo`) (`self.ClipSize`)))
      (bind _asfpplayer_character (cast `/Game/Assets/Player/FPPlayerCharacter` (`GameplayStatics.GetPlayerCharacter` 0)))
      (bind _output_get (set `/Game/Assets/Player/FPPlayerCharacter.IsReloading` true _asfpplayer_character))
      (else
        (set `self.Ammo` (`self.MaxAmmo`))
        (set `self.MaxAmmo` 0)
        (bind _asfpplayer_character_2 (cast `/Game/Assets/Player/FPPlayerCharacter` (`GameplayStatics.GetPlayerCharacter` 0)))
        (bind _output_get_2 (set `/Game/Assets/Player/FPPlayerCharacter.IsReloading` true _asfpplayer_character_2))))
    (return _output_get _output_get_2)))

(fn `UserConstructionScript`)